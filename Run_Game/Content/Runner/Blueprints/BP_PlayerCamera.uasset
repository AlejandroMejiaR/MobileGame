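; BP_PlayerCamera is the runner's follow camera, tracking the player forward while easing sideways between three lanes.
; Each Tick it moves the camera component to the player capsule's X plus a follow offset, with height taken directly from FollowLocation rather than the player.
; CalculateLaneLocation supplies Y by interpolating from the current camera position toward a target selected by LaneIndex and spaced by MoveAmount.
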(event `self.ReceiveTick`
  (params (DeltaSeconds :type "Float (single-precision)"))
  (bind _follow_location (`self.Follow_Location`))
  (bind _returnvalue_x (`KismetMathLibrary.BreakVector` (`SceneComponent.K2_GetComponentLocation` (`Character.CapsuleComponent` (`self.Player_Ref`)))))
  (`SceneComponent.K2_SetWorldLocation` (`self.CameraComponent`) (`KismetMathLibrary.MakeVector` (+ _returnvalue_x (.x (.location _follow_location))) (`self.CalculateLaneLocation`) (.z (.location _follow_location))) false false))

(fn `CalculateLaneLocation`
  (returns (Lane_Location :type "Float (double-precision)"))
  (bind _move_amount (`self.Move_Amount`))
  (bind (_returnvalue_x _returnvalue_y) (`KismetMathLibrary.BreakVector` (`SceneComponent.K2_GetComponentLocation` (`self.CameraComponent`))))
  (return (`KismetMathLibrary.FInterpTo` _returnvalue_y (select `int` (`self.Lane_Index`) :`0` (* _move_amount -1.0) :`1` 1.0 :`2` _move_amount) (`GameplayStatics.GetWorldDeltaSeconds`) 8.0)))

(fn `UserConstructionScript`)