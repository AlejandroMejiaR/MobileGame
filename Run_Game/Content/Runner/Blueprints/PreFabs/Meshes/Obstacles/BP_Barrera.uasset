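; BP_Barrera is a runner obstacle barrier that triggers the player's wall-obstacle death on contact.
; BeginPlay runs a validity check, retrying after short delays, then caches the player as a BP_RunCharacter.
; Tick polls the player's HyperRunning state, disabling collision on the barrier and death volume while it is active and restoring it otherwise.
; Overlapping DeathCollision calls DeathWallObstacle on the run character.
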(event `self.ReceiveBeginPlay`
  (`/Engine/EditorBlueprintResources/StandardMacros.IsValid` "/Game/Runner/Blueprints/BP_RunCharacter.BP_RunCharacter" :!label _label
    (:`Is Valid`
      (bind _asbp_run_character (cast `/Game/Runner/Blueprints/BP_RunCharacter` (`GameplayStatics.GetPlayerCharacter` 0)))
      (set `self.Player_Ref` _asbp_run_character))
    (:`Is Not Valid`
      (`KismetSystemLibrary.Delay` 0.01)
      (goto _label))))

(event `self.ReceiveTick`
  (params (DeltaSeconds :type "Float (single-precision)"))
  (if (`/Game/Runner/Blueprints/BP_RunCharacter.Hyper_Running?` (`self.Player_Ref`))
    (`PrimitiveComponent.SetCollisionEnabled` (`self.Barrera`) "NoCollision")
    (`PrimitiveComponent.SetCollisionEnabled` (`self.DeathCollision`) "NoCollision")
    (else
      (`PrimitiveComponent.SetCollisionEnabled` (`self.Barrera`) "QueryAndPhysics")
      (`PrimitiveComponent.SetCollisionEnabled` (`self.DeathCollision`) "QueryOnly"))))

(event `self.DeathCollision.OnComponentBeginOverlap`
  (params (OverlappedComponent :type "PrimitiveComponent Object Reference") (OtherActor :type "Actor Object Reference") (OtherComp :type "PrimitiveComponent Object Reference") (OtherBodyIndex :type Integer) (bFromSweep :type Boolean) (SweepResult :type "HitResult Structure (by ref)"))
  (bind _asbp_run_character (cast `/Game/Runner/Blueprints/BP_RunCharacter` OtherActor))
  (`/Game/Runner/Blueprints/BP_RunCharacter.DeathWallObstacle` _asbp_run_character))

(fn `UserConstructionScript`)