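; Base floor tile for an endless runner that dresses itself with random environment pieces and keeps the track going.
; On BeginPlay it walks five right and five left spawn points, adding one of five randomly chosen child actor components at each.
; When the run character overlaps SpawnCollision it asks the game mode to spawn a floor.
; Overlapping DestroyCollision destroys the tile.
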(event `self.ReceiveBeginPlay`
  (`self.Spawn_Environment`))

(event `self.SpawnCollision.OnComponentBeginOverlap`
  (params (OverlappedComponent :type "PrimitiveComponent Object Reference") (OtherActor :type "Actor Object Reference") (OtherComp :type "PrimitiveComponent Object Reference") (OtherBodyIndex :type Integer) (bFromSweep :type Boolean) (SweepResult :type "HitResult Structure (by ref)"))
  (cast `/Game/Runner/Blueprints/BP_RunCharacter` OtherActor)
  (`/Game/Runner/Blueprints/GM_Runner.SpawnFloor` (`self.Game_Mode_Ref`) 1))

(event `self.DestroyCollision.OnComponentBeginOverlap`
  (params (OverlappedComponent :type "PrimitiveComponent Object Reference") (OtherActor :type "Actor Object Reference") (OtherComp :type "PrimitiveComponent Object Reference") (OtherBodyIndex :type Integer) (bFromSweep :type Boolean) (SweepResult :type "HitResult Structure (by ref)"))
  (cast `/Game/Runner/Blueprints/BP_RunCharacter` OtherActor)
  (`self.K2_DestroyActor`))

(fn `Random_Env_Spawner`
  (switch `int` (`KismetMathLibrary.RandomIntegerInRange` 0 4)
    (:`0`
      (`AddComponent|NODE_AddChildActorComponent-0` :`RelativeTransform` (`self.Env_Spawn_Transform`)))
    (:`1`
      (`AddComponent|NODE_AddChildActorComponent-1` :`RelativeTransform` (`self.Env_Spawn_Transform`)))
    (:`2`
      (`AddComponent|NODE_AddChildActorComponent-2` :`RelativeTransform` (`self.Env_Spawn_Transform`)))
    (:`3`
      (`AddComponent|NODE_AddChildActorComponent-3` :`RelativeTransform` (`self.Env_Spawn_Transform`)))
    (:`4`
      (`AddComponent|NODE_AddChildActorComponent-4` :`RelativeTransform` (`self.Env_Spawn_Transform`)))))

(fn `Spawn_Environment`
  (`|ExecutionSequence`
    (:`then_0`
      (`|ExecutionSequence`
        (:`then_0`
          (set `self.Env_Spawn_Transform` (`SceneComponent.GetRelativeTransform` (`self.En_Spawn_Point_R1`)))
          (`self.Random_Env_Spawner`))
        (:`then_1`
          (set `self.Env_Spawn_Transform` (`SceneComponent.GetRelativeTransform` (`self.En_Spawn_Point_R2`)))
          (`self.Random_Env_Spawner`))
        (:`then_2`
          (set `self.Env_Spawn_Transform` (`SceneComponent.GetRelativeTransform` (`self.En_Spawn_Point_R3`)))
          (`self.Random_Env_Spawner`))
        (:`then_3`
          (set `self.Env_Spawn_Transform` (`SceneComponent.GetRelativeTransform` (`self.En_Spawn_Point_R4`)))
          (`self.Random_Env_Spawner`))
        (:`then_4`
          (set `self.Env_Spawn_Transform` (`SceneComponent.GetRelativeTransform` (`self.En_Spawn_Point_R5`)))
          (`self.Random_Env_Spawner`))))
    (:`then_1`
      (`|ExecutionSequence`
        (:`then_0`
          (set `self.Env_Spawn_Transform` (`SceneComponent.GetRelativeTransform` (`self.En_Spawn_Point_L1`)))
          (`self.Random_Env_Spawner`))
        (:`then_1`
          (set `self.Env_Spawn_Transform` (`SceneComponent.GetRelativeTransform` (`self.En_Spawn_Point_L2`)))
          (`self.Random_Env_Spawner`))
        (:`then_2`
          (set `self.Env_Spawn_Transform` (`SceneComponent.GetRelativeTransform` (`self.En_Spawn_Point_L3`)))
          (`self.Random_Env_Spawner`))
        (:`then_3`
          (set `self.Env_Spawn_Transform` (`SceneComponent.GetRelativeTransform` (`self.En_Spawn_Point_L4`)))
          (`self.Random_Env_Spawner`))
        (:`then_4`
          (set `self.Env_Spawn_Transform` (`SceneComponent.GetRelativeTransform` (`self.En_Spawn_Point_L5`)))
          (`self.Random_Env_Spawner`))))))

(fn `UserConstructionScript`)